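; BP_EnemyBase is a base enemy actor with simple health and lock-on targeting feedback.
; Lock-on events show or hide separate highlight and locked reticle components.
; Health starts at the maximum on BeginPlay, and a TakeDamage event applies fixed damage to itself through the engine damage system.
; AnyDamage subtracts incoming damage from current health and destroys the actor when it reaches zero.
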(event `/Game/ThirdPerson/Blueprints/BP_PlayerInterface.LockOnHighlightReticle`
  (params (`Hovering?` :type Boolean))
  (bind _highlightlockon (`self.HighlightLockOn`))
  (if `Hovering?`
    (`SceneComponent.SetHiddenInGame` _highlightlockon false false)
    (else
      (`SceneComponent.SetHiddenInGame` _highlightlockon true false))))

(event `/Game/ThirdPerson/Blueprints/BP_PlayerInterface.LockOnReticle`
  (params (`LockedOn?` :type Boolean))
  (bind _lockon (`self.LockOn`))
  (if `LockedOn?`
    (`SceneComponent.SetHiddenInGame` _lockon false false)
    (else
      (`SceneComponent.SetHiddenInGame` _lockon true false))))

(event `self.ReceiveBeginPlay`
  (set `self.CurrentHealth` (`self.MaxHeath`)))

(event `/Game/ThirdPerson/Blueprints/BP_EnemyData.TakeDamage`
  (`GameplayStatics.ApplyDamage` self 2.0))

(event `self.ReceiveAnyDamage`
  (params (Damage :type "Float (single-precision)") (DamageType :type "DamageType Object Reference") (InstigatedBy :type "Controller Object Reference") (DamageCauser :type "Actor Object Reference"))
  (bind _output_get (set `self.CurrentHealth` (- (`self.CurrentHealth`) (* Damage 1.0))))
  (if (<= _output_get 0)
    (`self.K2_DestroyActor`)))

(fn `UserConstructionScript`)