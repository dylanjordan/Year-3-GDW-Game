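; BP_EnemyBase is an enemy Character with health, a patrol route, selectable movement speeds and lock-on reticle display.
; Reticle events toggle hover and locked-on indicators, while GetPatrolRoute and SetMovementSpeed expose the route and set walk speed by movement state.
; TakeDamage applies fixed damage to itself, and AnyDamage subtracts health, destroying the actor at zero.
; Attack is a placeholder that prints and signals attack end; a forward launch node is left unconnected.
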(event `/Game/ThirdPerson/Blueprints/BP_PlayerInterface.LockOnHighlightReticle`
  (params (`Hovering?` :type Boolean))
  (bind _highlightlockon (`self.HighlightLockOn`))
  (if `Hovering?`
    (`SceneComponent.SetHiddenInGame` _highlightlockon false false)
    (else
      (`SceneComponent.SetHiddenInGame` _highlightlockon true false))))

(event `/Game/ThirdPerson/Blueprints/BP_PlayerInterface.LockOnReticle`
  (params (`LockedOn?` :type Boolean))
  (bind _lockon (`self.LockOn`))
  (if `LockedOn?`
    (`SceneComponent.SetHiddenInGame` _lockon false false)
    (else
      (`SceneComponent.SetHiddenInGame` _lockon true false))))

(event `self.ReceiveBeginPlay`
  (set `self.CurrentHealth` (`self.MaxHealth`)))

(event `/Game/ThirdPerson/Blueprints/BP_EnemyData.TakeDamage`
  (params (Actor :type "Actor Object Reference"))
  ;[1 1 1] Take Damage
  (`GameplayStatics.ApplyDamage` self 2.0 null Actor))

(event `self.ReceiveAnyDamage`
  (params (Damage :type "Float (single-precision)") (DamageType :type "DamageType Object Reference") (InstigatedBy :type "Controller Object Reference") (DamageCauser :type "Actor Object Reference"))
  ;[1 1 1] Damage Check
  (bind _output_get (set `self.CurrentHealth` (- (`self.CurrentHealth`) (* Damage 1.0))))
  (if (<= _output_get 0)
    (`self.K2_DestroyActor`)))

(event `Attack`
  ;[1 1 1] Enemy Attack
  (`KismetSystemLibrary.PrintText` "Enemy attacked")
  (`self.OnAttackEnd`))

(fn `GetPatrolRoute`
  (returns (PatrolRoute :type "/Game/Enemies/AI/PatrolRoute Object Reference"))
  ;[1 1 1] Gets Patrol Route
  (return (`self.PatrolRoute`)))

(fn `SetMovementSpeed`
  (params (Speed :type "/Game/Enemies/AI/Enums/E_MovementSpeed Enum" :default "NewEnumerator0"))
  (returns (SpeedValue :type "Float (double-precision)"))
  ;[1 1 1] Sets Movement Speed
  (bind _output_get (set `CharacterMovementComponent.MaxWalkSpeed` (select `/Game/Enemies/AI/Enums/E_MovementSpeed` Speed :`NewEnumerator1` 125.0 :`NewEnumerator2` 250.0 :`NewEnumerator3` 500.0 :!type "Float (single-precision)") (`self.CharacterMovement`)))
  (return _output_get))

(fn `UserConstructionScript`)