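; BP_BossZone is a trigger actor that shows a boss health bar while the player is inside its area.
; On begin overlap it confirms the overlapping actor is player 0's BP_ThirdPersonCharacter, then asks that character to spawn a health bar for the zone's BossRef.
; On end overlap the same check has the character remove the bar, so the zone only signals and the character handles the bar itself.
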(event `self.ReceiveActorBeginOverlap`
  (params (OtherActor :type "Actor Object Reference"))
  (bind _asbp_third_person_character (cast `/Game/ThirdPerson/Blueprints/BP_ThirdPersonCharacter` (`GameplayStatics.GetPlayerCharacter` 0)))
  (if (== _asbp_third_person_character OtherActor)
    (`/Game/ThirdPerson/Blueprints/BP_ThirdPersonCharacter.Spawn Boss HealthBar` _asbp_third_person_character (`self.BossRef`))))

(event `self.ReceiveActorEndOverlap`
  (params (OtherActor :type "Actor Object Reference"))
  (bind _asbp_third_person_character (cast `/Game/ThirdPerson/Blueprints/BP_ThirdPersonCharacter` (`GameplayStatics.GetPlayerCharacter` 0)))
  (if (== _asbp_third_person_character OtherActor)
    (`/Game/ThirdPerson/Blueprints/BP_ThirdPersonCharacter.Remove Boss HealthBar` _asbp_third_person_character)))

(fn `UserConstructionScript`)