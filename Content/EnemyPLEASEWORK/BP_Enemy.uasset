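; Enemy character Blueprint that roams at random, chases pawns it sees and attacks them up close.
; Roaming chains AI MoveTo calls to random navigable points, while PawnSensing starts the chase.
; DoOnce gates switch between jog and attack animations and speeds, with a timed reset for attacks.
; A retriggerable delay, refreshed by each sighting, drops the enemy back to slow walking and roaming.
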(event `self.ReceiveBeginPlay`
  (`self.MoveToRandomLocation`))

(event `MoveToRandomLocation`
  ;[1 1 1] Finds Random Location and then moves the character mesh to that location
  (bind _randomlocation (`NavigationSystemV1.K2_GetRandomLocationInNavigableRadius` (`self.K2_GetActorLocation`) 1000.0 null null))
  (`|AIMoveTo` self _randomlocation null
    (:`OnSuccess`
      (`self.MoveToRandomLocation`))))

(event `CanSprintAgain`
  (goto _label_2 :!via `Reset`))

(event `self.PawnSensing.OnSeePawn`
  (params (Pawn :type "Pawn Object Reference"))
  (`|ExecutionSequence`
    (:`then_0`
      (if (<= (`self.GetDistanceTo` Pawn) 300.0)
        (`/Engine/EditorBlueprintResources/StandardMacros.DoOnce` false :!label _label
          (:`Completed`
            (`SkeletalMeshComponent.PlayAnimation` (`self.Mesh`) "/Game/Enemies/AI/Animations/ZombieAttack_UE.ZombieAttack_UE" true)
            (set `CharacterMovementComponent.MaxWalkSpeed` 0.0 (`self.CharacterMovement`))
            (`self.CanSprintAgain`)
            (`KismetSystemLibrary.Delay` 3.0)
            (`self.CanAttackAgain`)))
        (else
          (`/Engine/EditorBlueprintResources/StandardMacros.DoOnce` false :!label _label_2
            (:`Completed`
              (`SkeletalMeshComponent.PlayAnimation` (`self.Mesh`) "/Game/Enemies/AI/Animations/JogForward_UE.JogForward_UE" true)
              (set `CharacterMovementComponent.MaxWalkSpeed` 600.0 (`self.CharacterMovement`)))))))
    (:`then_1`
      (`|AIMoveTo` self (0.0 0.0 0.0) Pawn
        (:`then`
          (`KismetSystemLibrary.RetriggerableDelay` 2.0)
          (`SkeletalMeshComponent.PlayAnimation` (`self.Mesh`) "/Game/Enemies/AI/Animations/MutantWalking_UE.MutantWalking_UE" true)
          (set `CharacterMovementComponent.MaxWalkSpeed` 130.0 (`self.CharacterMovement`))
          (`self.CanSprintAgain`)
          (`self.MoveToRandomLocation`))))))

(event `CanAttackAgain`
  (goto _label :!via `Reset`))

(fn `UserConstructionScript`)